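; Task 04 character Blueprint that exercises replication of a custom UObject and runtime-created components.
; On BeginPlay the server constructs BP_ObjectForReplication_04 and registers it with ObjectReplicationManager, while Tick prints its three variables in separate server and client colors.
; Server-call events randomize those variables or add a static mesh component, store it in DynamicComponent, then invoke a multicast event that adds another.
; The DynamicComponent OnRep is empty.
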(event `self.ReceiveBeginPlay`
  (if (`KismetSystemLibrary.IsServer`)
    (bind _returnvalue (`|GenericCreateObject` "/Game/Task_04/BP_ObjectForReplication_04.BP_ObjectForReplication_04_C" true 5.0 30))
    ;[1 1 1 0.2] Registred UObject for Replication
    (bind _output_get (set `self.Object for Replication` _returnvalue))
    (`ObjectReplicationManagerComponent.RegisterReplicatedObject` (`self.ObjectReplicationManager`) _output_get)))

(event `self.ReceiveTick`
  (params (DeltaSeconds :type "Float (single-precision)"))
  (bind _object_for_replication (`self.Object for Replication`))
  (bind _returnvalue (`KismetStringLibrary.Concat_StrStr` (`KismetStringLibrary.Conv_BoolToString` (`/Game/Task_04/BP_ObjectForReplication_04.Var1` _object_for_replication)) " | " (`KismetStringLibrary.Conv_DoubleToString` (`/Game/Task_04/BP_ObjectForReplication_04.Var2` _object_for_replication)) " | " (`KismetStringLibrary.Conv_IntToString` (`/Game/Task_04/BP_ObjectForReplication_04.Var3` _object_for_replication))))
  ;[0 0 0] Debug
  (if (`KismetSystemLibrary.IsServer`)
    (`KismetSystemLibrary.PrintString` _returnvalue true true (struct :`R` 1.0 :`B` 0.257534 :`A` 1.0) 0.0)
    (else
      (`KismetSystemLibrary.PrintString` _returnvalue true true (struct :`R` 1.0 :`G` 0.456295 :`A` 1.0) 0.0))))

(event `/Game/Task_04/BPI_WidgetToPlayerActor.AddValueServerCall`
  ;[0.3229 0.14 0.3161 0.5] Call Server Event | Change Value to UObject for Replication
  (`self.AddValueTo UObject`))

(event `AddValueTo UObject`
  (bind _object_for_replication (`self.Object for Replication`))
  ;[0.3229 0.14 0.3161 0.5] Call Server Event | Change Value to UObject for Replication
  (set `/Game/Task_04/BP_ObjectForReplication_04.Var1` (`KismetMathLibrary.RandomBool`) _object_for_replication)
  (set `/Game/Task_04/BP_ObjectForReplication_04.Var2` (`KismetMathLibrary.RandomFloatInRange` -50.0 50.0) _object_for_replication)
  (set `/Game/Task_04/BP_ObjectForReplication_04.Var3` (`KismetMathLibrary.RandomIntegerInRange` -10 10) _object_for_replication))

(event `/Game/Task_04/BPI_WidgetToPlayerActor.CreateComponentServerCall`
  ;[0.5781 0.2866 0 0.5] Call Multicast for client Replication | Create and Add Component
  (`self.Create Dynamic Component`))

(event `Create Dynamic Component`
  ;[0.5781 0.2866 0 0.5] Call Multicast for client Replication | Create and Add Component
  (bind _returnvalue (`AddComponent|NODE_AddStaticMeshComponent-1` :`bManualAttachment` true))
  (set `self.Dynamic Component` _returnvalue)
  (`self.Multicast Dynamic Content`))

(event `Multicast Dynamic Content`
  ;[0.5781 0.2866 0 0.5] Call Multicast for client Replication | Create and Add Component
  (bind _returnvalue (`AddComponent|NODE_AddStaticMeshComponent-3` :`bManualAttachment` true))
  (`KismetSystemLibrary.PrintString` (`KismetSystemLibrary.GetDisplayName` _returnvalue)))

(fn `OnRep_Dynamic Component`)

(fn `UserConstructionScript`)