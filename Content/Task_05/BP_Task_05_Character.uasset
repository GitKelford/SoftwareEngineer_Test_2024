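; Character for a task that moves along a spline actor at an input-adjustable speed, looping back to the start, and fires physics balls.
; While fire is held, a predicted projectile path is drawn with debug spheres and a hit-place marker spawned on press follows its end point.
; On release, a BP_PhysicBall spawns at the spawner component, launched along the control rotation with the same velocity as the prediction.
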(event `EnhancedInput|/Game/Basic/Input/IA_MovementSpeedUp`
  (params (ActionValue :type "Float (double-precision)") (ElapsedSeconds :type "Float (double-precision)") (TriggeredSeconds :type "Float (double-precision)") (InputAction :type "InputAction Object Reference" :default "/Game/Basic/Input/IA_MovementSpeedUp.IA_MovementSpeedUp"))
  ;[1 1 1 0.1] Speed Control
  (:`Triggered`
    (set `self.MovementSpeed` (+ (`self.MovementSpeed`) 10.0))))

(event `EnhancedInput|/Game/Basic/Input/IA_MovementSpeedDown`
  (params (ActionValue :type "Float (double-precision)") (ElapsedSeconds :type "Float (double-precision)") (TriggeredSeconds :type "Float (double-precision)") (InputAction :type "InputAction Object Reference" :default "/Game/Basic/Input/IA_MovementSpeedDown.IA_MovementSpeedDown"))
  ;[1 1 1 0.1] Speed Control
  (:`Triggered`
    (set `self.MovementSpeed` (- (`self.MovementSpeed`) 10.0))))

(event `self.ReceiveTick`
  (params (DeltaSeconds :type "Float (single-precision)"))
  (bind _spline (`/Game/Task_05/BP_Trajectory.Spline` (`self.SplineActor`)))
  ;[1 1 1 0.1] Mooving
  (bind _output_get (set `self.DistanceAlongSpline` (+ (`self.DistanceAlongSpline`) (* (`self.MovementSpeed`) DeltaSeconds))))
  (`self.K2_SetActorLocation` (`SplineComponent.GetLocationAtDistanceAlongSpline` _spline _output_get "World") true)
  (if (>= _output_get (`SplineComponent.GetSplineLength` _spline))
    (set `self.DistanceAlongSpline` 0.0)))

(event `EnhancedInput|/Game/Basic/Input/IA_Fire`
  (params (ActionValue :type Boolean) (ElapsedSeconds :type "Float (double-precision)") (TriggeredSeconds :type "Float (double-precision)") (InputAction :type "InputAction Object Reference" :default "/Game/Basic/Input/IA_Fire.IA_Fire"))
  ;[0 0 0] Prediction and shot processing
  ;;[1 0 0 0] Start Calculate and Fire
  (:`Triggered`
    (`self.Calculate Trajectory`))
  (:`Started`
    (bind _returnvalue (`|SpawnActorFromClass` "/Game/Task_05/BP_HitPlace.BP_HitPlace_C" (`KismetMathLibrary.Conv_VectorToTransform` (`self.HitLocation`)) "Undefined" "MultiplyWithRoot" null null))
    (set `self.HitActor` _returnvalue))
  (:`Completed`
    (`self.Fire`)))

(event `Calculate Trajectory`
  (bind (_returnvalue_roll _returnvalue_pitch _returnvalue_yaw) (`KismetMathLibrary.BreakRotator` (`self.GetControlRotation`)))
  ;[0 0 0] Prediction and shot processing
  ;;[1 0.5 0 0] Calculate Trajectory
  (bind (_outhit _outpathpositions) (`GameplayStatics.Blueprint_PredictProjectilePath_ByTraceChannel` (`SceneComponent.K2_GetComponentLocation` (`self.SpawnerProjectile`)) (* (`KismetMathLibrary.GetForwardVector` (`self.GetControlRotation`)) 1000) true 5.0 "ECC_Visibility" false (`|MakeArray` (`self.HitActor`) :!type "Actor Object Reference") "ForDuration"))
  (for _array_element _outpathpositions
    (`KismetSystemLibrary.DrawDebugSphere` _array_element 10.0 12 (struct :`R` 1.0 :`B` 0.022075 :`A` 1.0) 0.0 1.0))
  (bind _output_get (set `self.HitLocation` _array_element))
  (`self.K2_SetActorLocationAndRotation` (`self.HitActor`) _output_get (`KismetMathLibrary.MakeRotator` 0.0 0.0 _returnvalue_yaw) false false))

(event `Fire`
  (bind _spawnerprojectile (`self.SpawnerProjectile`))
  ;[0 0 0] Prediction and shot processing
  ;;[1 0 0 0] Fire
  (bind _returnvalue (`|SpawnActorFromClass` "/Game/Task_05/BP_PhysicBall.BP_PhysicBall_C" (`KismetMathLibrary.MakeTransform` (`SceneComponent.K2_GetComponentLocation` _spawnerprojectile) (`SceneComponent.K2_GetComponentRotation` _spawnerprojectile) (0.5 0.5 0.5)) "Undefined" "MultiplyWithRoot" null null))
  (`PrimitiveComponent.SetPhysicsLinearVelocity` (`/Game/Task_05/BP_PhysicBall.Sphere` _returnvalue) (* (`KismetMathLibrary.GetForwardVector` (`self.GetControlRotation`)) 1000) false "None"))

(fn `UserConstructionScript`)